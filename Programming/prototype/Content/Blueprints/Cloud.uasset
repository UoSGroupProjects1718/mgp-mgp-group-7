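; Cloud actor that drifts along negative X and loops back to the opposite side, likely as moving scenery.
; Each Tick moves the root component by a Speed variable, applied per frame without delta-time scaling.
; Once it passes the negative X limit, it teleports back to the positive X side with a random Y in a narrow band and Z reset to zero.
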(event EventBeginPlay)

(event Collision|EventActorBeginOverlap
  (params (OtherActor :type Actor%20Object%20Reference)))

(event EventTick
  (params (DeltaSeconds :type Float%20%28single-precision%29))
  (bind _defaultsceneroot (Variables|Default|GetDefaultSceneRoot))
  (bind _returnvalue (Transformation|GetWorldLocation _defaultsceneroot))
  (bind (_x _y _z) (Math|Vector|BreakVector _returnvalue))
  (if (< (.X (Math|Vector|BreakVector (Transformation|GetWorldLocation (Variables|Default|GetDefaultSceneRoot)))) -1e+03)
    (Transformation|SetWorldLocation (Variables|Default|GetDefaultSceneRoot) (Math|Vector|MakeVector 1e+03 (Math|Random|RandomFloatinRange -4.5e+02 -4e+02) 0.0) false false)
    (else
      (Transformation|SetWorldLocation (Variables|Default|GetDefaultSceneRoot) (Math|Vector|MakeVector (- _x (Variables|Default|GetSpeed)) _y _z) false false))))

(fn ConstructionScript)