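; Tree actor Blueprint that holds a randomized health value for a tree.
; SetHealth switches on TreeHealthBracket to roll TreeHealth within one of three preset ranges, while bracket 0 and any unmatched value use the LowerBound and UpperBound variables.
; Nothing in this file calls SetHealth, and the event graph holds only disabled events and an unconnected nested-random health assignment.
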(event Collision|EventActorBeginOverlap
  (params (OtherActor :type Actor%20Object%20Reference)))

(event EventTick
  (params (DeltaSeconds :type Float%20%28single-precision%29)))

(fn ConstructionScript)

(fn SetHealth
  (switch int (Variables|Default|GettreeHealthBracket)
    (:Default
      (Variables|Default|SettreeHealth (Math|Random|RandomIntegerinRange (Variables|Default|GetlowerBound) (Variables|Default|GetupperBound)) :!label _label))
    (:0
      (goto _label))
    (:1
      (Variables|Default|SettreeHealth (Math|Random|RandomIntegerinRange 20 40)))
    (:2
      (Variables|Default|SettreeHealth (Math|Random|RandomIntegerinRange 50 70)))
    (:3
      (Variables|Default|SettreeHealth (Math|Random|RandomIntegerinRange 80 100)))))