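; Notch is a Paper2D visual Blueprint that displays one of four notch sprites.
; Four custom events, SetNotch1 through SetNotch4, each swap the NotchSprite component to the matching sprite variable.
; It holds no state logic of its own: BeginPlay, overlap and Tick are disabled stubs and the construction script is empty.
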(event Custom|SetNotch1
  (Rendering|Components|Sprite|SetSprite (Variables|Default|GetNotchSprite) "/Game/Blueprint/notch_1_Sprite.notch_1_Sprite"))

(event Custom|SetNotch4
  (Rendering|Components|Sprite|SetSprite (Variables|Default|GetNotchSprite) "/Game/Blueprint/Notch_4_Sprite.Notch_4_Sprite"))

(event Custom|SetNotch2
  (Rendering|Components|Sprite|SetSprite (Variables|Default|GetNotchSprite) "/Game/Blueprint/Notch_2_Sprite.Notch_2_Sprite"))

(event Custom|SetNotch3
  (Rendering|Components|Sprite|SetSprite (Variables|Default|GetNotchSprite) "/Game/Blueprint/Notch_3_Sprite.Notch_3_Sprite"))

(event EventBeginPlay)

(event Collision|EventActorBeginOverlap
  (params (OtherActor :type Actor%20Object%20Reference)))

(event EventTick
  (params (DeltaSeconds :type Float%20%28single-precision%29)))

(fn ConstructionScript)