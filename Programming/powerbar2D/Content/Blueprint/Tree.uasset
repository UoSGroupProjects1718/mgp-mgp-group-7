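; Choppable tree actor that loses health when touched and shows the damage through a child Notch actor.
; BeginGame randomizes its health, then Tick moves a clamped power value by bar speed and direction until it reaches full.
; Each touch subtracts health scaled by that power and maps the remaining health fraction to one of four notch stages.
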(event Custom|BeginGame
  (Development|PrintString "Hello")
  (bind _output_get (Variables|Default|SetTreeHealth (Math|Random|RandomIntegerinRange 50 100)))
  (Variables|Default|SetTreeMaxHealth _output_get)
  (Variables|Default|SetGameReady true))

(event EventBeginPlay
  (bind _asnotch (Utilities|Casting|CastToNotch (Utilities|Array|Get(acopy) (Actor|GetAllChildActors false))))
  (Variables|Default|SetNotch _asnotch))

(event Collision|EventActorBeginOverlap
  (params (OtherActor :type Actor%20Object%20Reference)))

(event EventTick
  (params (DeltaSeconds :type Float%20%28single-precision%29))
  (bind _returnvalue (Utilities|Time|GetWorldDeltaSeconds))
  (bind _powerbarspeed (Variables|Default|GetPowerBarSpeed))
  (bind _returnvalue_2 (* _powerbarspeed _returnvalue))
  (if (Variables|Default|GetGameReady)
    (if (< (Variables|Default|GetCurrentPower) 1.0)
      (if (Variables|Default|GetPowerBarReverse)
        (Variables|Default|SetCurrentPower (Math|Float|Clamp(Float) (- (Variables|Default|GetCurrentPower) _returnvalue_2)))
        (else
          (Variables|Default|SetCurrentPower (Math|Float|Clamp(Float) (+ (Variables|Default|GetCurrentPower) _returnvalue_2))))))))

(event EventActorOnInputTouchBegin
  (params (FingerIndex :type ETouchIndex%20Enum :default "Touch1"))
  (bind _notch (Variables|Default|GetNotch))
  (Variables|Default|SetTreeHealth (- (Variables|Default|GetTreeHealth) (Math|Float|Truncate (* (Variables|Default|GetCurrentPower) (Variables|Default|GetPowerMultiplier)))))
  (Development|PrintString "Hello")
  (switch int (Math|Float|Truncate (* 4 (/ (Math|Conversions|ToFloat(Integer) (Variables|Default|GetTreeHealth)) (Math|Conversions|ToFloat(Integer) (Variables|Default|GetTreeMaxHealth)))))
    (:1
      (Default|SetNotch4 _notch))
    (:2
      (Default|SetNotch3 _notch))
    (:3
      (Default|SetNotch2 _notch))
    (:4
      (Default|SetNotch1 _notch))))

(fn ConstructionScript)