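; Notch is a Blueprint actor that displays one of four notch sprites through its NotchSprite component.
; Four custom events, SetNotch1 through SetNotch4, each swap in the matching sprite and reset the component's world scale to half size.
; BeginPlay, Tick, overlap and the construction script are empty, so the sprite changes only when one of these events is called.
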(event Custom|SetNotch1
  (Rendering|Components|Sprite|SetSprite (Variables|Default|GetNotchSprite) "/Game/Assets/Sprites/notch_1_Sprite.notch_1_Sprite")
  (Transformation|SetWorldScale3D (Variables|Default|GetNotchSprite) "0.500000,0.500000,0.500000"))

(event Custom|SetNotch4
  (Rendering|Components|Sprite|SetSprite (Variables|Default|GetNotchSprite) "/Game/Assets/Sprites/Notch_4_Sprite.Notch_4_Sprite")
  (Transformation|SetWorldScale3D (Variables|Default|GetNotchSprite) "0.500000,0.500000,0.500000"))

(event Custom|SetNotch2
  (Rendering|Components|Sprite|SetSprite (Variables|Default|GetNotchSprite) "/Game/Assets/Sprites/Notch_2_Sprite.Notch_2_Sprite")
  (Transformation|SetWorldScale3D (Variables|Default|GetNotchSprite) "0.500000,0.500000,0.500000"))

(event Custom|SetNotch3
  (Rendering|Components|Sprite|SetSprite (Variables|Default|GetNotchSprite) "/Game/Assets/Sprites/Notch_3_Sprite.Notch_3_Sprite")
  (Transformation|SetWorldScale3D (Variables|Default|GetNotchSprite) "0.500000,0.500000,0.500000"))

(event EventBeginPlay)

(event Collision|EventActorBeginOverlap
  (params (OtherActor :type Actor%20Object%20Reference)))

(event EventTick
  (params (DeltaSeconds :type Float%20%28single-precision%29)))

(fn ConstructionScript)