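; Background cloud actor that scrolls along negative X and recycles itself in an endless loop.
; Tick moves it a fixed step per frame, not scaled by delta time.
; Past the far X limit it jumps back to the start at a random height, and a counter toggles its Paper2D sprite between two cloud sets.
; The spawnCloud event is an empty stub.
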(event Custom|spawnCloud)

(event EventBeginPlay)

(event Collision|EventActorBeginOverlap
  (params (OtherActor :type Actor%20Object%20Reference)))

(event EventTick
  (params (DeltaSeconds :type Float%20%28single-precision%29))
  (bind _returnvalue (Transformation|GetActorLocation))
  (Transformation|SetActorLocation (+ (Transformation|GetActorLocation) (Math|Vector|MakeVector -5.0 0.0 0.0)) false false)
  (if (not (> (.x _returnvalue) -1.4e+03))
    (Transformation|SetActorLocation (Math|Vector|MakeVector 1e+03 (.y _returnvalue) (Math|Random|RandomFloatinRange 1.2e+03 1.56e+03)) false false)
    (Math|Integer|IncrementInt (Variables|Default|GetnCloud)
      (:%20%20
        (if (== (Variables|Default|GetnCloud) 2)
          (Variables|Default|SetnCloud 0))
        (if (== (Variables|Default|GetnCloud) 1)
          (Rendering|Components|Sprite|SetSprite (Variables|Default|GetcloudSprite) "/Game/Assets/Sprites/Cloud_Set_2_Sprite.Cloud_Set_2_Sprite")
          (else
            (Rendering|Components|Sprite|SetSprite (Variables|Default|GetcloudSprite) "/Game/Assets/Sprites/Cloud_Set_1_Sprite.Cloud_Set_1_Sprite")))))))

(fn ConstructionScript)