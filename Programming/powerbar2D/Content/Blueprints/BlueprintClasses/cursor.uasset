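; Cursor actor that slides back and forth along the X axis, apparently as the marker of a timing bar.
; Tick moves it by Forward each frame without delta-time scaling, and overlapping a "bar"-tagged actor reverses its direction.
; Overlaps with "sweetspot" and "catch-up" actors toggle matching flags, and entering the sweetspot also calls Vibrate on the 2D side-scroller player character.
; The F key handler does nothing.
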(event EventBeginPlay)

(event Collision|EventActorBeginOverlap
  (params (OtherActor :type Actor%20Object%20Reference))
  (if (Actor|ActorHasTag OtherActor "bar")
    (Variables|Default|Setforward (* (Variables|Default|Getforward) -1.0))
    (elif (Actor|ActorHasTag OtherActor "sweetspot")
      (Variables|Default|Setsweetspot true)
      (bind _as2dside_scroller_character (Utilities|Casting|CastTo2DSideScrollerCharacter (Game|GetPlayerCharacter 0)))
      (Default|Vibrate _as2dside_scroller_character)
      (elif (Actor|ActorHasTag OtherActor "catch-up")
        (Variables|Default|Setcatch-up true)))))

(event EventTick
  (params (DeltaSeconds :type Float%20%28single-precision%29))
  (Transformation|SetActorLocation (+ (Transformation|GetActorLocation) (Math|Vector|MakeVector (Variables|Default|Getforward) 0.0 0.0)) false false))

(event Collision|EventActorEndOverlap
  (params (OtherActor :type Actor%20Object%20Reference))
  (if (Actor|ActorHasTag OtherActor "sweetspot")
    (Variables|Default|Setsweetspot false)
    (elif (Actor|ActorHasTag OtherActor "catch-up")
      (Variables|Default|Setcatch-up false))))

(event Input|KeyboardEvents|F
  (params (Key :type Key%20Structure))
  (:Pressed
    (if true
      _)))

(fn ConstructionScript)